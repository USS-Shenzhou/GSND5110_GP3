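; BP_Worm is a player-possessed inchworm pawn that crawls by arching and stretching its body.
; Arch pulls the tail toward the head and Stretch pushes the head along the clamped, input-steered yaw, with ground line traces setting both heights.
; Each tick, UpdateBody places the actor at the tail and shapes body segments as curves, deriving hump height from constant body length.
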(event Input|EnhancedActionEvents|EnhancedInputActionIA_WormArch
  (params (ActionValue :type Boolean) (ElapsedSeconds :type Float%20%28double-precision%29) (TriggeredSeconds :type Float%20%28double-precision%29) (InputAction :type Input%20Action%20Object%20Reference :default "/Game/GP3/Input/IA_WormArch.IA_WormArch"))
  (CallFunction|ArchStep))

(event Input|EnhancedActionEvents|EnhancedInputActionIA_WormStretch
  (params (ActionValue :type Boolean) (ElapsedSeconds :type Float%20%28double-precision%29) (TriggeredSeconds :type Float%20%28double-precision%29) (InputAction :type Input%20Action%20Object%20Reference :default "/Game/GP3/Input/IA_WormStretch.IA_WormStretch"))
  (CallFunction|StretchStep))

(event Input|EnhancedActionEvents|EnhancedInputActionIA_WormHeadTurn
  (params (ActionValue :type Vector%202D%20Structure) (ElapsedSeconds :type Float%20%28double-precision%29) (TriggeredSeconds :type Float%20%28double-precision%29) (InputAction :type Input%20Action%20Object%20Reference :default "/Game/GP3/Input/IA_WormHeadTurn.IA_WormHeadTurn"))
  (CallFunction|TurnHead ActionValue))

(event Collision|EventActorBeginOverlap
  (params (OtherActor :type Actor%20Object%20Reference)))

(event EventPossessed
  (params (NewController :type Controller%20Object%20Reference))
  (CallFunction|RegisterInput))

(event EventBeginPlay
  (CallFunction|InitWorm))

(event EventTick
  (params (DeltaSeconds :type Float%20%28single-precision%29))
  (CallFunction|UpdateBody))

(fn ConstructionScript)

(fn InitWorm
  (bind _returnvalue (Transformation|GetActorLocation))
  (bind _returnvalue_2 (Transformation|GetActorForwardVector))
  (bind _returnvalue_3 (Transformation|GetActorRotation))
  (bind _meshradius (Variables|Default|GetMeshRadius))
  (bind _bodylength (Variables|Default|GetBodyLength))
  (bind _meshlength (Variables|Default|GetMeshLength))
  (bind (_x _y) (Math|Vector|BreakVector _returnvalue_2))
  (bind (_x_2 _y_2 _z) (Math|Vector|BreakVector _returnvalue))
  (bind _yaw (Math|Rotator|BreakRotator _returnvalue_3))
  (bind _returnvalue_4 (/ _bodylength _meshlength))
  (bind _returnvalue_5 (* _bodylength 0.5))
  (bind _returnvalue_6 (Math|Vector2D|MakeVector2D _returnvalue_4 _returnvalue_4))
  (bind _returnvalue_7 (* _meshradius _returnvalue_4))
  (bind _returnvalue_8 (* _x _returnvalue_5))
  (bind _returnvalue_9 (* _y _returnvalue_5))
  (bind _returnvalue_10 (* _x _returnvalue_5))
  (bind _returnvalue_11 (* _y _returnvalue_5))
  (bind _returnvalue_12 (- _x_2 _returnvalue_8))
  (bind _returnvalue_13 (- _y_2 _returnvalue_9))
  (bind _returnvalue_14 (+ _x_2 _returnvalue_10))
  (bind _returnvalue_15 (+ _y_2 _returnvalue_11))
  (CallFunction|InitSegment (Variables|Default|GetBody) _returnvalue_6 _returnvalue_7)
  (CallFunction|InitSegment (Variables|Default|GetBodySegment1) _returnvalue_6 _returnvalue_7)
  (CallFunction|InitSegment (Variables|Default|GetBodySegment2) _returnvalue_6 _returnvalue_7)
  (CallFunction|InitSegment (Variables|Default|GetBodySegment3) _returnvalue_6 _returnvalue_7)
  (bind _groundheight (CallFunction|GroundZ (Math|Vector|MakeVector _returnvalue_12 _returnvalue_13 _z)))
  (Variables|Default|SetTailLocation (Math|Vector|MakeVector _returnvalue_12 _returnvalue_13 _groundheight))
  (bind _groundheight_2 (CallFunction|GroundZ (Math|Vector|MakeVector _returnvalue_14 _returnvalue_15 _z)))
  (Variables|Default|SetHeadLocation (Math|Vector|MakeVector _returnvalue_14 _returnvalue_15 _groundheight_2))
  (Variables|Default|SetCameraYaw _yaw)
  (Variables|Default|SetHeadYaw _yaw)
  (CallFunction|UpdateBody))

(fn RegisterInput
  (Input|AddMappingContext (PlayerController|LocalPlayerSubsystems|GetEnhancedInputLocalPlayerSubsystem (Game|GetPlayerController 0)) "/Game/GP3/Input/IMC_Worm.IMC_Worm" 0 "(bIgnoreAllPressedKeysUntilRelease=True,bForceImmediately=False,bNotifyUserSettings=False)"))

(fn ArchStep
  (bind _headlocation (Variables|Default|GetHeadLocation))
  (bind _bodylength (Variables|Default|GetBodyLength))
  (bind _minchordratio (Variables|Default|GetMinChordRatio))
  (bind (_x _y) (Math|Vector|BreakVector _headlocation))
  (bind _returnvalue (* _bodylength _minchordratio))
  (bind _groundheight (CallFunction|GroundZ (Math|Vector|MakeVector (- _x (* (.X (Math|Vector|BreakVector (Class|KismetMathLibrary|VectorNormal2D (- _headlocation (Variables|Default|GetTailLocation)) 0.0001))) (Math|Float|Max(Float) (- (Math|Vector|Distance2D(Vector) _headlocation (Variables|Default|GetTailLocation)) (* (* (* (- _bodylength _returnvalue) (Variables|Default|GetArchRate)) (Utilities|Time|GetWorldDeltaSeconds)) (Math|Float|SelectFloat 0.0 1.0 (Input|EnhancedActionValues|GetIA_WormStretch)))) _returnvalue))) (- _y (* (.Y (Math|Vector|BreakVector (Class|KismetMathLibrary|VectorNormal2D (- _headlocation (Variables|Default|GetTailLocation)) 0.0001))) (Math|Float|Max(Float) (- (Math|Vector|Distance2D(Vector) _headlocation (Variables|Default|GetTailLocation)) (* (* (* (- _bodylength _returnvalue) (Variables|Default|GetArchRate)) (Utilities|Time|GetWorldDeltaSeconds)) (Math|Float|SelectFloat 0.0 1.0 (Input|EnhancedActionValues|GetIA_WormStretch)))) _returnvalue))) (.Z (Math|Vector|BreakVector (Variables|Default|GetTailLocation))))))
  (Variables|Default|SetTailLocation (Math|Vector|MakeVector (- _x (* (.X (Math|Vector|BreakVector (Class|KismetMathLibrary|VectorNormal2D (- _headlocation (Variables|Default|GetTailLocation)) 0.0001))) (Math|Float|Max(Float) (- (Math|Vector|Distance2D(Vector) _headlocation (Variables|Default|GetTailLocation)) (* (* (* (- _bodylength _returnvalue) (Variables|Default|GetArchRate)) (Utilities|Time|GetWorldDeltaSeconds)) (Math|Float|SelectFloat 0.0 1.0 (Input|EnhancedActionValues|GetIA_WormStretch)))) _returnvalue))) (- _y (* (.Y (Math|Vector|BreakVector (Class|KismetMathLibrary|VectorNormal2D (- _headlocation (Variables|Default|GetTailLocation)) 0.0001))) (Math|Float|Max(Float) (- (Math|Vector|Distance2D(Vector) _headlocation (Variables|Default|GetTailLocation)) (* (* (* (- _bodylength _returnvalue) (Variables|Default|GetArchRate)) (Utilities|Time|GetWorldDeltaSeconds)) (Math|Float|SelectFloat 0.0 1.0 (Input|EnhancedActionValues|GetIA_WormStretch)))) _returnvalue))) _groundheight)))

(fn StretchStep
  (bind _returnvalue (Utilities|Time|GetWorldDeltaSeconds))
  (bind _returnvalue_2 (Input|EnhancedActionValues|GetIA_WormArch))
  (bind _archrate (Variables|Default|GetArchRate))
  (bind _headyaw (Variables|Default|GetHeadYaw))
  (bind _taillocation (Variables|Default|GetTailLocation))
  (bind _bodylength (Variables|Default|GetBodyLength))
  (bind _minchordratio (Variables|Default|GetMinChordRatio))
  (bind _returnvalue_3 (Math|Float|SelectFloat 0.0 1.0 _returnvalue_2))
  (bind (_x _y) (Math|Vector|BreakVector _taillocation))
  (bind _returnvalue_4 (* _bodylength _minchordratio))
  (bind _returnvalue_5 (- _bodylength _returnvalue_4))
  (bind _returnvalue_6 (* _returnvalue_5 _archrate))
  (bind _returnvalue_7 (* _returnvalue_6 _returnvalue))
  (bind _returnvalue_8 (* _returnvalue_7 _returnvalue_3))
  (bind _groundheight (CallFunction|GroundZ (Math|Vector|MakeVector (+ _x (* (.X (Math|Vector|BreakVector (Class|KismetMathLibrary|VectorNormal2D (- (Math|Vector|MakeVector (+ (.X (Math|Vector|BreakVector (Variables|Default|GetHeadLocation))) (* (Math|Trig|Cos(Degrees) _headyaw) _returnvalue_8)) (+ (.Y (Math|Vector|BreakVector (Variables|Default|GetHeadLocation))) (* (Math|Trig|Sin(Degrees) _headyaw) _returnvalue_8)) (.Z (Math|Vector|BreakVector (Variables|Default|GetHeadLocation)))) _taillocation) 0.0001))) (Math|Float|Min(Float) (Math|Vector|Distance2D(Vector) (Math|Vector|MakeVector (+ (.X (Math|Vector|BreakVector (Variables|Default|GetHeadLocation))) (* (Math|Trig|Cos(Degrees) _headyaw) _returnvalue_8)) (+ (.Y (Math|Vector|BreakVector (Variables|Default|GetHeadLocation))) (* (Math|Trig|Sin(Degrees) _headyaw) _returnvalue_8)) (.Z (Math|Vector|BreakVector (Variables|Default|GetHeadLocation)))) _taillocation) _bodylength))) (+ _y (* (.Y (Math|Vector|BreakVector (Class|KismetMathLibrary|VectorNormal2D (- (Math|Vector|MakeVector (+ (.X (Math|Vector|BreakVector (Variables|Default|GetHeadLocation))) (* (Math|Trig|Cos(Degrees) _headyaw) _returnvalue_8)) (+ (.Y (Math|Vector|BreakVector (Variables|Default|GetHeadLocation))) (* (Math|Trig|Sin(Degrees) _headyaw) _returnvalue_8)) (.Z (Math|Vector|BreakVector (Variables|Default|GetHeadLocation)))) _taillocation) 0.0001))) (Math|Float|Min(Float) (Math|Vector|Distance2D(Vector) (Math|Vector|MakeVector (+ (.X (Math|Vector|BreakVector (Variables|Default|GetHeadLocation))) (* (Math|Trig|Cos(Degrees) _headyaw) _returnvalue_8)) (+ (.Y (Math|Vector|BreakVector (Variables|Default|GetHeadLocation))) (* (Math|Trig|Sin(Degrees) _headyaw) _returnvalue_8)) (.Z (Math|Vector|BreakVector (Variables|Default|GetHeadLocation)))) _taillocation) _bodylength))) (.Z (Math|Vector|BreakVector (Variables|Default|GetHeadLocation))))))
  (Variables|Default|SetHeadLocation (Math|Vector|MakeVector (+ _x (* (.X (Math|Vector|BreakVector (Class|KismetMathLibrary|VectorNormal2D (- (Math|Vector|MakeVector (+ (.X (Math|Vector|BreakVector (Variables|Default|GetHeadLocation))) (* (Math|Trig|Cos(Degrees) _headyaw) _returnvalue_8)) (+ (.Y (Math|Vector|BreakVector (Variables|Default|GetHeadLocation))) (* (Math|Trig|Sin(Degrees) _headyaw) _returnvalue_8)) (.Z (Math|Vector|BreakVector (Variables|Default|GetHeadLocation)))) _taillocation) 0.0001))) (Math|Float|Min(Float) (Math|Vector|Distance2D(Vector) (Math|Vector|MakeVector (+ (.X (Math|Vector|BreakVector (Variables|Default|GetHeadLocation))) (* (Math|Trig|Cos(Degrees) _headyaw) _returnvalue_8)) (+ (.Y (Math|Vector|BreakVector (Variables|Default|GetHeadLocation))) (* (Math|Trig|Sin(Degrees) _headyaw) _returnvalue_8)) (.Z (Math|Vector|BreakVector (Variables|Default|GetHeadLocation)))) _taillocation) _bodylength))) (+ _y (* (.Y (Math|Vector|BreakVector (Class|KismetMathLibrary|VectorNormal2D (- (Math|Vector|MakeVector (+ (.X (Math|Vector|BreakVector (Variables|Default|GetHeadLocation))) (* (Math|Trig|Cos(Degrees) _headyaw) _returnvalue_8)) (+ (.Y (Math|Vector|BreakVector (Variables|Default|GetHeadLocation))) (* (Math|Trig|Sin(Degrees) _headyaw) _returnvalue_8)) (.Z (Math|Vector|BreakVector (Variables|Default|GetHeadLocation)))) _taillocation) 0.0001))) (Math|Float|Min(Float) (Math|Vector|Distance2D(Vector) (Math|Vector|MakeVector (+ (.X (Math|Vector|BreakVector (Variables|Default|GetHeadLocation))) (* (Math|Trig|Cos(Degrees) _headyaw) _returnvalue_8)) (+ (.Y (Math|Vector|BreakVector (Variables|Default|GetHeadLocation))) (* (Math|Trig|Sin(Degrees) _headyaw) _returnvalue_8)) (.Z (Math|Vector|BreakVector (Variables|Default|GetHeadLocation)))) _taillocation) _bodylength))) _groundheight))
  (CallFunction|ClampHeadYaw))

(fn TurnHead
  (params (LookInput :type Vector%202D%20Structure))
  (Variables|Default|SetCameraYaw (+ (Variables|Default|GetCameraYaw) (* (.X (Math|Vector2D|BreakVector2D LookInput)) (Variables|Default|GetHeadTurnSensitivity))))
  (CallFunction|ClampHeadYaw))

(fn ClampHeadYaw
  (bind _maxheadyaw (Variables|Default|GetMaxHeadYaw))
  (bind _headlocation (Variables|Default|GetHeadLocation))
  (bind _taillocation (Variables|Default|GetTailLocation))
  (bind (_x _y) (Math|Vector|BreakVector _headlocation))
  (bind (_x_2 _y_2) (Math|Vector|BreakVector _taillocation))
  (bind _returnvalue (- _y _y_2))
  (bind _returnvalue_2 (- _x _x_2))
  (bind _returnvalue_3 (Class|KismetMathLibrary|DegAtan2 _returnvalue _returnvalue_2))
  (Variables|Default|SetHeadYaw (+ _returnvalue_3 (Math|Float|Clamp(Float) (Math|Rotator|NormalizeAxis (- (Variables|Default|GetCameraYaw) _returnvalue_3)) (* _maxheadyaw -1.0) _maxheadyaw))))

(fn GroundZ
  (params (Location :type Vector))
  (bind (_outhit _returnvalue) (Collision|LineTraceByChannel (+ Location (Math|Vector|MakeVector 0.0 0.0 1e+01)) (- Location (Math|Vector|MakeVector 0.0 0.0 1e+03)) "TraceTypeQuery1" false 0 "None"))
  (return (Math|Float|SelectFloat (.Z (Math|Vector|BreakVector (.ImpactPoint (Collision|BreakHitResult _outhit)))) (.Z (Math|Vector|BreakVector Location)) (and _returnvalue (not (.bInitialOverlap (Collision|BreakHitResult _outhit)))))))

(fn UpdateBody
  (bind _returnvalue (Math|Vector|MakeVector 0.0 0.0 0.0))
  (bind _headlocation (Variables|Default|GetHeadLocation))
  (bind _taillocation (Variables|Default|GetTailLocation))
  (bind _bodylength (Variables|Default|GetBodyLength))
  (bind _footratio (Variables|Default|GetFootRatio))
  (bind _headyaw (Variables|Default|GetHeadYaw))
  (bind _cameraboom (Variables|Default|GetCameraBoom))
  (bind _returnvalue_2 (- _headlocation _taillocation))
  (bind _returnvalue_3 (* _bodylength _footratio))
  (bind _returnvalue_4 (Math|Vector|MakeVector _returnvalue_3 0.0 0.0))
  (bind (_x _y _z) (Math|Vector|BreakVector _returnvalue_2))
  (bind _returnvalue_5 (Math|Vector|VectorLengthXY _returnvalue_2))
  (bind _returnvalue_6 (Math|Vector|MakeVector _returnvalue_3 0.0 0.0))
  (bind _returnvalue_7 (* _returnvalue_3 2.0))
  (bind _returnvalue_8 (Class|KismetMathLibrary|DegAtan2 _y _x))
  (bind _returnvalue_9 (Math|Vector|MakeVector _returnvalue_5 0.0 _z))
  (bind _returnvalue_10 (- _bodylength _returnvalue_7))
  (bind _returnvalue_11 (* _z 0.5))
  (bind _returnvalue_12 (- _headyaw _returnvalue_8))
  (bind _returnvalue_13 (* _returnvalue_10 _returnvalue_10))
  (bind _returnvalue_14 (* _returnvalue_10 0.5))
  (bind _returnvalue_15 (Math|Rotator|NormalizeAxis _returnvalue_12))
  (bind _returnvalue_16 (Math|Trig|Cos(Degrees) _returnvalue_15))
  (bind _returnvalue_17 (Math|Trig|Sin(Degrees) _returnvalue_15))
  (bind _returnvalue_18 (* _returnvalue_3 _returnvalue_16))
  (bind _returnvalue_19 (* _returnvalue_3 _returnvalue_17))
  (bind _returnvalue_20 (* _returnvalue_3 _returnvalue_16))
  (bind _returnvalue_21 (* _returnvalue_3 _returnvalue_17))
  (bind _returnvalue_22 (Math|Vector|MakeVector _returnvalue_20 _returnvalue_21 0.0))
  (bind _returnvalue_23 (- _returnvalue_5 _returnvalue_18))
  (bind _returnvalue_24 (* _returnvalue_19 -1.0))
  (bind _returnvalue_25 (Math|Vector|MakeVector _returnvalue_23 _returnvalue_24 _z))
  (bind _returnvalue_26 (- _returnvalue_23 _returnvalue_3))
  (bind _returnvalue_27 (+ _returnvalue_3 _returnvalue_23))
  (bind _returnvalue_28 (* _returnvalue_24 0.5))
  (bind _returnvalue_29 (Math|Vector|MakeVector _returnvalue_26 _returnvalue_24 0.0))
  (bind _returnvalue_30 (* _returnvalue_27 0.5))
  (bind _returnvalue_31 (Math|Vector|VectorLengthXY _returnvalue_29))
  (bind _returnvalue_32 (Class|KismetMathLibrary|VectorNormal2D _returnvalue_29 0.0001))
  (bind (_x_2 _y_2) (Math|Vector|BreakVector _returnvalue_32))
  (bind _returnvalue_33 (* _returnvalue_31 _returnvalue_31))
  (bind _returnvalue_34 (* _returnvalue_31 0.5))
  (bind _returnvalue_35 (- _returnvalue_13 _returnvalue_33))
  (bind _returnvalue_36 (Math|Float|Max(Float) _returnvalue_35 0.0))
  (bind _returnvalue_37 (Math|Float|Sqrt _returnvalue_36))
  (bind _returnvalue_38 (* _returnvalue_37 0.5))
  (bind _returnvalue_39 (+ _returnvalue_11 _returnvalue_38))
  (bind _returnvalue_40 (/ _returnvalue_38 _returnvalue_14))
  (bind _returnvalue_41 (Math|Float|Clamp(Float) _returnvalue_40 0.0 1.0))
  (bind _returnvalue_42 (Math|Vector|MakeVector _returnvalue_30 _returnvalue_28 _returnvalue_39))
  (bind _returnvalue_43 (* _returnvalue_41 1.5))
  (bind _returnvalue_44 (+ _returnvalue_43 1.0))
  (bind _returnvalue_45 (* _returnvalue_34 _returnvalue_44))
  (bind _returnvalue_46 (Math|Vector|MakeVector _returnvalue_45 0.0 0.0))
  (bind _returnvalue_47 (* _returnvalue_45 _x_2))
  (bind _returnvalue_48 (* _returnvalue_45 _y_2))
  (bind _returnvalue_49 (* _returnvalue_45 _returnvalue_16))
  (bind _returnvalue_50 (* _returnvalue_45 _returnvalue_17))
  (bind _returnvalue_51 (Math|Vector|MakeVector _returnvalue_47 _returnvalue_48 0.0))
  (bind _returnvalue_52 (Math|Vector|MakeVector _returnvalue_49 _returnvalue_50 0.0))
  (Transformation|SetActorLocationAndRotation _taillocation (Math|Rotator|MakeRotator 0.0 0.0 _returnvalue_8))
  (CallFunction|ApplySegmentCurve (Variables|Default|GetBody) _returnvalue _returnvalue_4 _returnvalue_6 _returnvalue_4 _returnvalue_25 _returnvalue_22 _returnvalue_9 _returnvalue_22)
  (CallFunction|ApplySegmentCurve (Variables|Default|GetBodySegment1) _returnvalue_6 _returnvalue_46 _returnvalue_42 _returnvalue_51 _returnvalue_42 _returnvalue_51 _returnvalue_25 _returnvalue_52)
  (CallFunction|ApplySegmentCurve (Variables|Default|GetBodySegment2) _returnvalue_42 _returnvalue_51 _returnvalue_25 _returnvalue_52 _returnvalue_6 _returnvalue_46 _returnvalue_42 _returnvalue_51)
  (CallFunction|ApplySegmentCurve (Variables|Default|GetBodySegment3) _returnvalue_25 _returnvalue_22 _returnvalue_9 _returnvalue_22 _returnvalue _returnvalue_4 _returnvalue_6 _returnvalue_4)
  (Transformation|SetRelativeLocation _cameraboom (Math|Vector|MakeVector (* _returnvalue_5 0.5) 0.0 (+ (* _z 0.5) 2e+01)) false false)
  (Transformation|SetRelativeRotation _cameraboom (Math|Rotator|MakeRotator 0.0 -25.0 (Math|Rotator|NormalizeAxis (- (Variables|Default|GetCameraYaw) _returnvalue_8))) false false))

(fn InitSegment
  (params (Segment :type Spline%20Mesh%20Component%20Object%20Reference) (CrossSectionScale :type Vector%202D%20Structure) (LiftZ :type Float%20%28double-precision%29))
  (SplineMesh|SetStartScale Segment CrossSectionScale true :!class /Script/Engine.SplineMeshComponent)
  (SplineMesh|SetEndScale Segment CrossSectionScale true :!class /Script/Engine.SplineMeshComponent)
  (Transformation|SetRelativeLocation Segment (Math|Vector|MakeVector 0.0 0.0 LiftZ) false false))

(fn ApplySegmentCurve
  (params (Segment :type Spline%20Mesh%20Component%20Object%20Reference) (ForwardStart :type Vector) (ForwardStartTangent :type Vector) (ForwardEnd :type Vector) (ForwardEndTangent :type Vector) (MirrorStart :type Vector) (MirrorStartTangent :type Vector) (MirrorEnd :type Vector) (MirrorEndTangent :type Vector))
  (bind _bheadatmeshend (Variables|Default|GetbHeadAtMeshEnd))
  (SplineMesh|SetStartandEnd Segment (Math|Vector|SelectVector ForwardStart MirrorEnd _bheadatmeshend) (Math|Vector|SelectVector ForwardStartTangent (Math|Vector|NegateVector MirrorEndTangent) _bheadatmeshend) (Math|Vector|SelectVector ForwardEnd MirrorStart _bheadatmeshend) (Math|Vector|SelectVector ForwardEndTangent (Math|Vector|NegateVector MirrorStartTangent) _bheadatmeshend) true :!class /Script/Engine.SplineMeshComponent))